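; HeadPickableBP is a pickable item, named for a head, that reacts to being collected.
; OnCollection spawns the actor class stored in InventoryInfo at player 0's transform, even if colliding.
; It then prints the item count of the player CharacterBP's inventory as debug output.
; A disconnected loop for printing class names never runs.
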(event EventOnCollection
  (bind _returnvalue (Game|GetPlayerCharacter 0))
  (bind _asactor (Utilities|Casting|CastToActorClass (.Class (Utilities|Struct|BreakInventoryItemInfo (Variables|Default|GetInventoryInfo)))))
  (Game|SpawnActorfromClass _asactor (Transformation|GetWorldTransform _returnvalue) true 0)
  (bind _ascharacter_bp (Utilities|Casting|CastToCharacterBP _returnvalue))
  (Development|PrintString (Utilities|String|ToString(Integer) (Utilities|Array|Length (Variables|/Script/Untitled.Inventory|GetItems (Variables|/Script/Untitled.CharacterBase|GetInventory _ascharacter_bp))))))

(fn ConstructionScript)